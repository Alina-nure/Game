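; Player character that moves on world X/Y, fires cannonballs and persists its position in a local MySQL database.
; Each tick, control rotation follows a yaw computed from velocity, which also aims spawned cannonballs.
; Shooting spends Armo (ammo) and uses a timer as its cooldown.
; LoadFromDB swaps in the UI and restores position and ammo by username through nested queries, while EndPlay writes back only the position.
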(event OnComponentBeginOverlap(CapsuleComponent)
  (params (OverlappedComponent :type Primitive%20Component%20Object%20Reference) (OtherActor :type Actor%20Object%20Reference) (OtherComp :type Primitive%20Component%20Object%20Reference) (OtherBodyIndex :type Integer) (bFromSweep :type Boolean) (SweepResult :type Hit%20Result%20Structure%20%28by%20ref%29)))

(event Input|EnhancedActionEvents|EnhancedInputActionIA_Shoot
  (params (ActionValue :type Boolean) (ElapsedSeconds :type Float%20%28double-precision%29) (TriggeredSeconds :type Float%20%28double-precision%29) (InputAction :type Input%20Action%20Object%20Reference :default "/Game/Input/Actions/IA_Shoot.IA_Shoot"))
  (if (<= (Utilities|Time|GetTimerRemainingTimebyHandle (Variables|Default|Gettimer)) 0.0)
    (CallFunction|Shooting)
    (bind _returnvalue (Utilities|Time|SetTimerbyFunctionName 0 "Update Animation" 2.0))
    (Variables|Default|Settimer _returnvalue)))

(event Input|EnhancedActionEvents|EnhancedInputActionIA_Move
  (params (ActionValue :type Vector%202D%20Structure) (ElapsedSeconds :type Float%20%28double-precision%29) (TriggeredSeconds :type Float%20%28double-precision%29) (InputAction :type Input%20Action%20Object%20Reference :default "/Game/Input/Actions/IA_Move.IA_Move"))
  (bind (_x _y) (Math|Vector2D|BreakVector2D ActionValue))
  (Pawn|Input|AddMovementInput "1.000000,0.000000,0.000000" _x false)
  (Pawn|Input|AddMovementInput "0.000000,-1.000000,0.000000" _y false))

(event EventBeginPlay
  (bind _asplayer_controller (Utilities|Casting|CastToPlayerController (Pawn|GetController)))
  (Input|AddMappingContext (PlayerController|LocalPlayerSubsystems|GetEnhancedInputLocalPlayerSubsystem _asplayer_controller) "/Game/Input/IMC_Platforming.IMC_Platforming" 0 "(bIgnoreAllPressedKeysUntilRelease=True,bForceImmediately=False,bNotifyUserSettings=False)"))

(event EventTick
  (params (DeltaSeconds :type Float%20%28single-precision%29))
  (CallFunction|UpdateAnimation))

(event EventEndPlay
  (params (EndPlayReason :type EEndPlayReason%20Enum :default "Destroyed"))
  (bind _returnvalue (Transformation|GetActorLocation))
  (bind (_x _y _z) (Math|Vector|BreakVector _returnvalue))
  (bind _connection (Utilities|MySQLConnect "127.0.0.1" "root" "" "game")
    (:Success
      (Utilities|MySQLExecuteQuery (Utilities|String|Append (Variables|Default|Getfirst_part) (Variables|Default|Getcoordinate_X) (Utilities|String|ToString(Float) _x) (Variables|Default|Getsecond_part) (Variables|Default|GetUSER_NAME) (Variables|Default|Getend_FIND)) _connection
        (:Success
          (Utilities|MySQLExecuteQuery (Utilities|String|Append (Variables|Default|Getfirst_part) (Variables|Default|Getcoordinate_Y) (Utilities|String|ToString(Float) _y) (Variables|Default|Getsecond_part) (Variables|Default|GetUSER_NAME) (Variables|Default|Getend_FIND)) _connection
            (:Success
              (Utilities|MySQLExecuteQuery (Utilities|String|Append (Variables|Default|Getfirst_part) (Variables|Default|Getcoordinate_Z) (Utilities|String|ToString(Float) _z) (Variables|Default|Getsecond_part) (Variables|Default|GetUSER_NAME) (Variables|Default|Getend_FIND)) _connection))))))))

(fn ConstructionScript)

(fn UpdateAnimation
  (bind _returnvalue (CallFunction|RotationAngle "0, 0, 0"))
  (Pawn|SetControlRotation (Pawn|GetController) _returnvalue))

(fn RotationAngle
  (params (NewParam :type Rotator))
  (bind _returnvalue (Transformation|GetVelocity))
  (bind _returnvalue_2 (Transformation|GetVelocity))
  (bind _returnvalue_3 (Transformation|GetVelocity))
  (bind _returnvalue_4 (Transformation|GetVelocity))
  (bind _returnvalue_5 (Transformation|GetVelocity))
  (bind _returnvalue_6 (> (.y _returnvalue_2) 0.0))
  (if (> (.x _returnvalue_2) 0.0)
    (if _returnvalue_6
      (return (Math|Rotator|MakeRotator 0.0 0.0 (Class|KismetMathLibrary|DegAtan (/ (.y _returnvalue_3) (.x _returnvalue_3)))))
      (else
        (return (Math|Rotator|MakeRotator 0.0 0.0 (- 3.6e+02 (Class|KismetMathLibrary|DegAtan (/ (* (.y _returnvalue_4) -1.0) (.x _returnvalue_4))))))))
    (elif _returnvalue_6
      (return (Math|Rotator|MakeRotator 0.0 0.0 (- 1.8e+02 (Class|KismetMathLibrary|DegAtan (/ (.y _returnvalue) (* (.x _returnvalue) -1.0))))))
      (else
        (return (Math|Rotator|MakeRotator 0.0 0.0 (+ 1.8e+02 (Class|KismetMathLibrary|DegAtan (/ (* (.y _returnvalue_5) -1.0) (* (.x _returnvalue_5) -1.0))))))))))

(fn Shooting
  (if (> (Variables|Default|GetArmo) 0)
    (bind _returnvalue (CallFunction|RotationAngle "0, 0, 0"))
    (bind _returnvalue_2 (Game|SpawnActorfromClass "/Game/Blueprints/CanonBall.CanonBall_C" (Math|Transform|MakeTransform (Transformation|GetActorLocation) _returnvalue) "AlwaysSpawn" "MultiplyWithRoot" 0 0))
    (Utilities|Array|AddUnique (Variables|Default|GetCanonBalls) _returnvalue_2)
    (bind _result (Math|Integer|DecrementInt (Variables|Default|GetArmo))
      (:%20%20
        (Variables|Default|SetArmo _result)))))

(fn LoadfromDB
  (params (NewParam1 :type String))
  (Development|PrintString "LoadFromDB" true true "(R=1.000000,G=0.000000,B=0.022392,A=1.000000)" 1e+01)
  (Viewport|RemoveAllWidgets)
  (bind _returnvalue (UserInterface|CreateWidget "/Game/Blueprints/Player/UI.UI_C"))
  (UserInterface|Viewport|AddtoViewport _returnvalue 0)
  (bind _connection (Utilities|MySQLConnect "127.0.0.1" "root" "" "game")
    (:Success
      (bind _result_rows (Utilities|MySQLExecuteQuerywithResult (Utilities|String|Append (Variables|Default|Getfirst_FIND_X) NewParam1 (Variables|Default|Getend_FIND)) _connection)
        (:Success
          (for _array_element _result_rows
            (for _array_element_2 (.fields _array_element)
              (bind _result_rows_2 (Utilities|MySQLExecuteQuerywithResult (Utilities|String|Append (Variables|Default|Getfirst_FIND_Y) NewParam1 (Variables|Default|Getend_FIND)) _connection)
                (:Success
                  (for _array_element_3 _result_rows_2
                    (for _array_element_4 (.fields _array_element_3)
                      (bind _result_rows_3 (Utilities|MySQLExecuteQuerywithResult (Utilities|String|Append (Variables|Default|Getfirst_FIND_Z) NewParam1 (Variables|Default|Getend_FIND)) _connection)
                        (:Success
                          (for _array_element_5 _result_rows_3
                            (for _array_element_6 (.fields _array_element_5)
                              (Transformation|SetActorLocation (Math|Vector|MakeVector (Math|Conversions|ToFloat(Integer) (.value _array_element_2)) (Math|Conversions|ToFloat(Integer) (.value _array_element_4)) (Math|Conversions|ToFloat(Integer) (.value _array_element_6))) false false)
                              (bind _result_rows_4 (Utilities|MySQLExecuteQuerywithResult (Utilities|String|Append (Variables|Default|Getfirst_FIND_ARMO) NewParam1 (Variables|Default|Getend_FIND)) _connection)
                                (:Success
                                  (for _array_element_7 _result_rows_4
                                    (for _array_element_8 (.fields _array_element_7)
                                      (Variables|Default|SetArmo (Math|Conversions|ToInteger(Byte) (.value _array_element_8)))
                                      (Variables|Default|SetUSER_NAME NewParam1))))))))))))))))))))