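; CanonBall is a flipbook-sprite cannonball projectile that flies across the XY plane along its yaw.
; Each Tick it teleports a fixed step using the yaw's cosine and sine, without delta-time scaling, or destroys itself if yaw equals exactly 180.
; Leaving a hard-coded rectangle switches the sprite to the Explosion flipbook but does not stop or destroy it.
; Overlap events are empty, so it has no hit logic.
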(event OnComponentBeginOverlap(CapsuleComponent)
  (params (OverlappedComponent :type Primitive%20Component%20Object%20Reference) (OtherActor :type Actor%20Object%20Reference) (OtherComp :type Primitive%20Component%20Object%20Reference) (OtherBodyIndex :type Integer) (bFromSweep :type Boolean) (SweepResult :type Hit%20Result%20Structure%20%28by%20ref%29)))

(event EventBeginPlay)

(event Collision|EventActorBeginOverlap
  (params (OtherActor :type Actor%20Object%20Reference)))

(event EventTick
  (params (DeltaSeconds :type Float%20%28single-precision%29))
  (bind _returnvalue (Transformation|GetActorLocation))
  (bind _returnvalue_2 (Transformation|GetActorLocation))
  (bind _returnvalue_3 (Transformation|GetActorRotation))
  (bind (_x _y _z) (Math|Vector|BreakVector _returnvalue))
  (bind (_x_2 _y_2) (Math|Vector|BreakVector _returnvalue_2))
  (bind _yaw (Math|Rotator|BreakRotator _returnvalue_3))
  (if (== _yaw 1.8e+02)
    (Actor|DestroyActor)
    (else
      (Transformation|Teleport (Math|Vector|MakeVector (+ _x (* (Math|Trig|Cos(Degrees) _yaw) 3e+01)) (+ _y (* (Math|Trig|Sin(Degrees) _yaw) 3e+01)) _z) _returnvalue_3)
      (if (or (or (< _x_2 -1e+02) (> _x_2 7e+03)) (or (< _y_2 -1e+02) (> _y_2 3.5e+03)))
        (Sprite|SetFlipbook (Variables|Default|GetSprite) "/Game/PaperAssets/Character/FlipBooks/explosion.explosion")))))

(fn ConstructionScript)